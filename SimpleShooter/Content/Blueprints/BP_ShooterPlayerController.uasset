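; BP_ShooterPlayerController is a player controller that owns the shooter's HUD and end-of-game screens.
; On BeginPlay it creates WBP_HUD and adds it to the viewport.
; The GameOverUI event removes the HUD and shows WBP_WinScreen or WBP_LoseScreen based on the Victory flag, passing RestartDelay to the chosen screen.
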(event EventBeginPlay
  (bind _returnvalue (UserInterface|CreateWidget "/Game/Blueprints/UI/WBP_HUD.WBP_HUD_C"))
  (bind _output_get (Variables|Default|SetHUD _returnvalue))
  (UserInterface|Viewport|AddtoViewport _output_get 0))

(event EventGameOverUI
  (params (bVictory :type Boolean))
  (bind _restartdelay (Variables|Default|GetRestartDelay))
  (Widget|RemovefromParent (Variables|Default|GetHUD))
  (if bVictory
    (bind _returnvalue (UserInterface|CreateWidget "/Game/Blueprints/UI/WBP_WinScreen.WBP_WinScreen_C" 0 _restartdelay))
    (UserInterface|Viewport|AddtoViewport _returnvalue 0)
    (else
      (bind _returnvalue_2 (UserInterface|CreateWidget "/Game/Blueprints/UI/WBP_LoseScreen.WBP_LoseScreen_C" 0 _restartdelay))
      (UserInterface|Viewport|AddtoViewport _returnvalue_2 0))))

(fn ConstructionScript)